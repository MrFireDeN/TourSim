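; Test bench actor that seats an AI avatar on one of its Smart Object slots, tracking a capacity of two.
; FindSeat queries sit slots within its enlarged bounds, claims a random one, starts its gameplay behavior and snaps the avatar onto it.
; Found, unavailable and freed outcomes fire dispatcher calls.
; While seats remain, a separate EnterClaimHandle slot is marked free after seating or freeing.
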(event Custom|Find%20Seat
  (params (Avatar :type Actor%20Object%20Reference))
  (bind (_origin _boxextent) (Collision|GetActorBounds false false))
  (Variables|Default|SetAvatar Avatar)
  (bind (_outresults _returnvalue) (Class|SmartObjectSubsystem|FindSmartObjectsBP (Subsystems|GetSmartObjectSubsystem) (Utilities|Struct|MakeSmartObjectRequest (Class|KismetMathLibrary|MakeBoxwithOrigin _origin (* _boxextent 1.1)) (Utilities|Struct|MakeSmartObjectRequestFilter "(GameplayTags=((TagName=\"SmartObject.User\")))" "Normal" "(TokenStreamVersion=0,TagDictionary=((TagName=\"SmartObject.Action.Sit\")),QueryTokenStream=(0,1,1,1,0),UserDescription=\"\",AutoDescription=\" ANY( SmartObject.Action.Sit )\")")) (Variables|Default|GetAvatar)))
  (if _returnvalue
    (bind _returnvalue_2 (Class|SmartObjectBlueprintFunctionLibrary|MarkSmartObjectSlotasClaimed (.SlotHandle (Utilities|Struct|BreakSmartObjectRequestResult (.OutItem (Utilities|Array|Random _outresults)))) (Variables|Default|GetAvatar) "Normal"))
    (|UseSmartObjectwithGameplayBehavior (AI|GetAIController (Variables|Default|GetAvatar)) _returnvalue_2 true "Normal"
      (:then
        (if (.ReturnValue (Class|SmartObjectSubsystem|GetSlotTransform (Subsystems|GetSmartObjectSubsystem) _returnvalue_2))
          (Transformation|SetActorLocationAndRotation (Variables|Default|GetAvatar) (.Location (Math|Transform|BreakTransform (.OutSlotTransform (Class|SmartObjectSubsystem|GetSlotTransform (Subsystems|GetSmartObjectSubsystem) _returnvalue_2)))) (.Rotation (Math|Transform|BreakTransform (.OutSlotTransform (Class|SmartObjectSubsystem|GetSlotTransform (Subsystems|GetSmartObjectSubsystem) _returnvalue_2)))))
          (Default|CallOnFoundSeat (Variables|Default|GetAvatar))
          (Math|Integer|IncrementInt (Variables|Default|GetSeatsTaken)
            (:%20%20
              (if (CallFunction|HasFreeSeats)
                (Class|SmartObjectBlueprintFunctionLibrary|MarkSmartObjectSlotasFree (Variables|Default|GetEnter%20Claim%20Handle)))))
          (else
            ;[0.15 0 0 0.5] Unavaible
            (Default|CallOnUnavaibleSeat (Variables|Default|GetAvatar)))))
      (:OnSucceeded
        (CallFunction|FreeSeat))
      (:OnFailed
        (Default|CallOnFreeSeat false :!label _label))
      (:OnMoveToFailed
        (goto _label)))
    (else
      ;[0.15 0 0 0.5] Unavaible
      (Default|CallOnUnavaibleSeat (Variables|Default|GetAvatar)))))

(event Custom|FreeSeat
  (Math|Integer|DecrementInt (Variables|Default|GetSeatsTaken)
    (:%20%20
      (Default|CallOnFreeSeat true)
      (if (CallFunction|HasFreeSeats)
        (Class|SmartObjectBlueprintFunctionLibrary|MarkSmartObjectSlotasFree (Variables|Default|GetEnter%20Claim%20Handle))))))

(event EventBeginPlay)

(event Collision|EventActorBeginOverlap
  (params (OtherActor :type Actor%20Object%20Reference)))

(event EventTick
  (params (DeltaSeconds :type Float%20%28single-precision%29)))

(fn ConstructionScript)

(fn HasFreeSeats
  (return (< (Variables|Default|GetSeatsTaken) 2)))