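; BP_NPC is a tourist NPC that randomizes its look and personal profile when play begins.
; It creates dynamic body and hair materials and fills their color parameters with random colors through a SetParameter helper.
; It then builds a Preferences tourist snapshot with random ID, money, needs, attraction weights, price sensitivity and spawn source, taking a name from TouristNamePoolSubsystem or falling back to a default.
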(event EventBeginPlay
  (bind _returnvalue (Math|Random|RandomInteger 10000))
  (bind _returnvalue_2 (Subsystems|GetTouristNamePoolSubsystem))
  (bind _mesh (Variables|Character|GetMesh))
  (bind (_outname _returnvalue_3) (Class|TouristNamePoolSubsystem|TryGetName _returnvalue_2 _returnvalue))
  (bind _returnvalue_4 (Rendering|Material|CreateDynamicMaterialInstance _mesh 0 (Rendering|Material|GetMaterial _mesh 0) "Body" :!class /Script/Engine.PrimitiveComponent))
  (CallFunction|SetParameter _returnvalue_4 "TopColor")
  (CallFunction|SetParameter _returnvalue_4 "BottomColor")
  (bind _returnvalue_5 (Rendering|Material|CreateDynamicMaterialInstance (Variables|Character|GetMesh) 1 (Rendering|Material|GetMaterial _mesh 1) "Hair" :!class /Script/Engine.PrimitiveComponent))
  (CallFunction|SetParameter _returnvalue_5 "HairColor")
  (Variables|Default|SetPreferences (Utilities|Struct|MakeTouristSnapshot _returnvalue (select _returnvalue_3 _outname "John") (Math|Random|RandomIntegerinRange 1000 10000) (Math|Random|RandomFloatinRange 0.2 0.5) (Math|Random|RandomFloatinRange 0.2 0.5) (Math|Random|RandomFloatinRange 0.2 0.5) (Math|Random|RandomFloatinRange 0.2 0.5) (Math|Random|RandomFloatinRange 0.2 0.5) (Math|Random|RandomFloatinRange 0.2 0.5) (Math|Random|RandomFloatinRange 0.2 0.5) (.OutItem (Utilities|Array|Random (Utilities|Array|MakeArray 0 1))))))

(event Collision|EventActorBeginOverlap
  (params (OtherActor :type Actor%20Object%20Reference)))

(event EventTick
  (params (DeltaSeconds :type Float%20%28single-precision%29)))

(fn ConstructionScript)

(fn IsMale
  (return (Variables|Default|GetSex)))

(fn IsFemale
  (return (not (Variables|Default|GetSex))))

(fn SetParameter
  (params (Material :type Material%20Instance%20Dynamic%20Object%20Reference) (ParameterName :type Name))
  (Rendering|Material|SetVectorParameterValue Material ParameterName (Math|Color|MakeColor (Math|Random|RandomFloat) (Math|Random|RandomFloat) (Math|Random|RandomFloat)) :!class /Script/Engine.MaterialInstanceDynamic))