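; Gameplay Behavior that makes a BP_NPC play a sitting animation when triggered.
; It casts the avatar to BP_NPC and uses IsFemale to choose between the male sit montage and a female montage named as a test asset.
; The behavior ends when the montage completes, blends out or is interrupted.
; If the cast fails, it stops without calling EndBehavior.
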(event GameplayBehavior|EventOnTriggeredCharacter
  (params (Avatar :type Character%20Object%20Reference) (Config :type Gameplay%20Behavior%20Config%20Object%20Reference) (SmartObjectOwner :type Actor%20Object%20Reference))
  (bind _output_get (Variables|Default|SetAvatar Avatar))
  (bind _asbp_npc (Utilities|Casting|CastToBP_NPC _output_get))
  (if (Default|IsFemale _asbp_npc)
    (Animation|Montage|PlayMontage (Variables|/Script/Engine.Character|GetMesh _output_get) "/Game/Project/AI/Animations/AM_Female_Test.AM_Female_Test"
      (:OnCompleted
        _)
      (:OnBlendOut
        _)
      (:OnInterrupted
        _))
    (GameplayBehavior|EndBehavior (Variables|Default|GetAvatar))
    (else
      (Animation|Montage|PlayMontage (Variables|/Script/Engine.Character|GetMesh _output_get) "/Game/Project/AI/Animations/AM_Sit_Male.AM_Sit_Male"
        (:OnCompleted
          _)
        (:OnBlendOut
          _)
        (:OnInterrupted
          _))
      (GameplayBehavior|EndBehavior (Variables|Default|GetAvatar)))))