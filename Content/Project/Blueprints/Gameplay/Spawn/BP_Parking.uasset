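; Parking prop Blueprint that fills three car slots with randomly chosen static meshes.
; Each of the Car1, Car2 and Car3 components gets an independent random pick from the Cars array, so duplicates are possible.
; The same randomization runs in the construction script and again on BeginPlay, so the in-game layout can differ from the editor preview.
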(event EventBeginPlay
  (Components|StaticMesh|SetStaticMesh (Variables|Default|GetCar1) (.OutItem (Utilities|Array|Random (Variables|Default|GetCars))))
  (Components|StaticMesh|SetStaticMesh (Variables|Default|GetCar2) (.OutItem (Utilities|Array|Random (Variables|Default|GetCars))))
  (Components|StaticMesh|SetStaticMesh (Variables|Default|GetCar3) (.OutItem (Utilities|Array|Random (Variables|Default|GetCars)))))

(event Collision|EventActorBeginOverlap
  (params (OtherActor :type Actor%20Object%20Reference)))

(event EventTick
  (params (DeltaSeconds :type Float%20%28single-precision%29)))

(fn ConstructionScript
  (Components|StaticMesh|SetStaticMesh (Variables|Default|GetCar1) (.OutItem (Utilities|Array|Random (Variables|Default|GetCars))))
  (Components|StaticMesh|SetStaticMesh (Variables|Default|GetCar2) (.OutItem (Utilities|Array|Random (Variables|Default|GetCars))))
  (Components|StaticMesh|SetStaticMesh (Variables|Default|GetCar3) (.OutItem (Utilities|Array|Random (Variables|Default|GetCars)))))