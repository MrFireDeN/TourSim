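; BP_TouristParking is a parking prop that shows three cars with randomly chosen meshes.
; SetRandomCars gives each of the three car mesh components an independent random pick from the Cars array, so duplicates are possible.
; It runs in the Construction Script and again on BeginPlay, so the cars are re-randomized when play starts.
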(event EventBeginPlay
  (CallFunction|SetRandomCars))

(event Collision|EventActorBeginOverlap
  (params (OtherActor :type Actor%20Object%20Reference)))

(event EventTick
  (params (DeltaSeconds :type Float%20%28single-precision%29)))

(fn ConstructionScript
  (CallFunction|SetRandomCars))

(fn SetRandomCars
  (Components|StaticMesh|SetStaticMesh (Variables|Default|GetCar1) (.OutItem (Utilities|Array|Random (Variables|Default|GetCars))))
  (Components|StaticMesh|SetStaticMesh (Variables|Default|GetCar2) (.OutItem (Utilities|Array|Random (Variables|Default|GetCars))))
  (Components|StaticMesh|SetStaticMesh (Variables|Default|GetCar3) (.OutItem (Utilities|Array|Random (Variables|Default|GetCars)))))