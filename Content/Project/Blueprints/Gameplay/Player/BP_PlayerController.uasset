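; Player controller that switches between the player character and a spectator pawn, and lets the player inspect tourists.
; Axis input drives whichever pawn is possessed; toggling spawns a spectator above the frozen character or destroys it on return, then broadcasts the mode.
; A mouse toggle enables cursor clicks that trace for Mass agent actors.
; A looping timer polls the selected tourist's snapshot and broadcasts it, removing the info widget when the snapshot fails.
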(event Custom|UdpateTouristInfo
  (bind _currenttourist (Variables|Default|GetCurrentTourist))
  (Utilities|IsValid _currenttourist
    (:Is%20Valid
      (bind (_outsnapshot _returnvalue) (Class|TouristBlueprintLibrary|GetTouristSnapshotfromActor _currenttourist))
      (if _returnvalue
        (Default|CallOnUpdateTouristInfo _outsnapshot)
        (else
          (Utilities|Time|ClearandInvalidateTimerbyHandle (Variables|Default|GetTouristInfoTimer) :!label _label)
          (Widget|RemovefromParent (Variables|Default|GetTouristInfoWidget)))))
    (:Is%20Not%20Valid
      (goto _label))))

(event EventBeginPlay
  (Variables|Default|SetPlayerCharacter (Game|GetPlayerCharacter 0))
  (bind _returnvalue (UserInterface|CreateWidget "/Game/Project/UI/UMG_Help.UMG_Help_C" self))
  (UserInterface|Viewport|AddtoViewport _returnvalue 0)
  (bind _returnvalue_2 (UserInterface|CreateWidget "/Game/Project/UI/UMG_TouristPrefs.UMG_TouristPrefs_C" self))
  (Variables|Default|SetTouristInfoWidget _returnvalue_2))

(event EventTick
  (params (DeltaSeconds :type Float%20%28single-precision%29)))

(event Input|ActionEvents|InputActionTogglePawn
  (params (Key :type Key%20Structure :default "None"))
  ;[0.15 0 0 0.5] Toggle Player Mode
  (:Pressed
    (Utilities|FlowControl|DoOnce false :!label _label
      (:Completed
        (if (== (Variables|Default|GetPlayerCharacter) (Pawn|GetControlledPawn))
          (CallFunction|SwitchtoSpectator)
          (else
            (CallFunction|SwitchtoCharacter))))))
  (:Released
    (goto _label Reset)))

(event Input|ActionEvents|InputActionToggleMouse
  (params (Key :type Key%20Structure :default "None"))
  (bind _self self)
  ;[0.15 0.09346 0 0.5] Toggle Mouse
  (:Pressed
    (Utilities|FlowControl|DoOnce false :!label _label
      (:Completed
        (bind _output_get (Variables|Default|SetbShowMouseCursor (not (Variables|Default|GetbShowMouseCursor))))
        (if _output_get
          (Input|SetInputModeGameandUI _self 0 "LockAlways" true true)
          (Variables|Default|SetbEnableClickEvents true)
          (else
            (Input|SetInputModeGameOnly _self true)
            (Variables|Default|SetbEnableClickEvents false))))))
  (:Released
    (goto _label Reset)))

(event Input|AxisEvents|InputAxisMove_Forward
  (params (AxisValue :type Float%20%28single-precision%29))
  (bind _returnvalue (Pawn|GetControlledPawn))
  ;[0 0.0399 0.15 0.5] Movemnet and Camera
  (Utilities|IsValid _returnvalue
    (:Is%20Valid
      (Pawn|Input|AddMovementInput _returnvalue (* AxisValue (Math|Vector|GetForwardVector (Math|Rotator|MakeRotator 0.0 0.0 (.yaw (Pawn|GetControlRotation :!class /Script/Engine.Controller))))) 1.0 false))))

(event Input|AxisEvents|InputAxisMove_Right
  (params (AxisValue :type Float%20%28single-precision%29))
  (bind _returnvalue (Pawn|GetControlledPawn))
  ;[0 0.0399 0.15 0.5] Movemnet and Camera
  (Utilities|IsValid _returnvalue
    (:Is%20Valid
      (Pawn|Input|AddMovementInput _returnvalue (* AxisValue (Math|Vector|GetRightVector (Math|Rotator|MakeRotator 0.0 0.0 (.yaw (Pawn|GetControlRotation :!class /Script/Engine.Controller))))) 1.0 false))))

(event Input|AxisEvents|InputAxisLook_Up
  (params (AxisValue :type Float%20%28single-precision%29))
  (bind _returnvalue (Pawn|GetControlledPawn))
  ;[0 0.0399 0.15 0.5] Movemnet and Camera
  (Utilities|IsValid _returnvalue
    (:Is%20Valid
      (Pawn|Input|AddControllerPitchInput _returnvalue AxisValue))))

(event Input|AxisEvents|InputAxisLook_Right
  (params (AxisValue :type Float%20%28single-precision%29))
  (bind _returnvalue (Pawn|GetControlledPawn))
  ;[0 0.0399 0.15 0.5] Movemnet and Camera
  (Utilities|IsValid _returnvalue
    (:Is%20Valid
      (Pawn|Input|AddControllerYawInput _returnvalue AxisValue))))

(event Input|MouseEvents|LeftMouseButton
  (params (Key :type Key%20Structure :default "None"))
  (bind _object_types (Variables|Default|GetObject%20Types))
  (bind _hitresult (Class|PlayerController|GetHitResultUnderCursorforObjects _object_types true))
  (bind (_bblockinghit _binitialoverlap _time _distance _location _impactpoint _normal _impactnormal _physmat _hitactor) (Collision|BreakHitResult _hitresult))
  (:Pressed
    (Utilities|FlowControl|DoOnce false :!label _label
      (:Completed
        (if (Variables|Default|GetbEnableClickEvents)
          (if _bblockinghit
            (Variables|Default|SetCurrentTourist _hitactor)
            (Utilities|IsValid (Actor|GetComponentbyClass _hitactor "/Script/MassActors.MassAgentComponent")
              (:Is%20Valid
                (bind _returnvalue (Class|TouristBlueprintLibrary|GetTouristSnapshotfromActor _hitactor))
                (Utilities|Time|ClearandInvalidateTimerbyHandle (Variables|Default|GetTouristInfoTimer))
                (if _returnvalue
                  (UserInterface|Viewport|AddtoViewport (Variables|Default|GetTouristInfoWidget) 0)
                  (bind _returnvalue_2 (Utilities|Time|SetTimerbyEvent (delegate Custom|UdpateTouristInfo) 0.2 true))
                  (Variables|Default|SetTouristInfoTimer _returnvalue_2)
                  (else
                    (Widget|RemovefromParent (Variables|Default|GetTouristInfoWidget)))))))))))
  (:Released
    (goto _label Reset)))

(fn ConstructionScript)

(fn SwitchtoCharacter
  (bind _playercharacter (Variables|Default|GetPlayerCharacter))
  (Pawn|Possess _playercharacter)
  (Pawn|Components|CharacterMovement|SetMovementMode (Variables|/Script/Engine.Character|GetCharacterMovement _playercharacter) "MOVE_Walking" 0)
  (Actor|DestroyActor (Variables|Default|GetPlayerSpectator))
  (bind _output_get (Variables|Default|SetCurrentPlayerMode 0))
  (Default|CallOnChangePlayerMode _output_get))

(fn SwitchtoSpectator
  (bind _playercharacter (Variables|Default|GetPlayerCharacter))
  (bind _returnvalue (Game|SpawnActorfromClass "/Game/Project/Blueprints/Gameplay/Player/BP_PlayerSpecator.BP_PlayerSpecator_C" (Math|Transform|MakeTransform (+ (Transformation|GetActorLocation _playercharacter) "0.000000,0.000000,500.000000") (Pawn|GetControlRotation :!class /Script/Engine.Controller) "1.000000,1.000000,1.000000") "Undefined" "MultiplyWithRoot" self 0))
  (bind _output_get (Variables|Default|SetPlayerSpectator _returnvalue))
  (Pawn|Possess _output_get)
  (Pawn|Components|CharacterMovement|SetMovementMode (Variables|/Script/Engine.Character|GetCharacterMovement _playercharacter) "MOVE_None" 0)
  (bind _output_get_2 (Variables|Default|SetCurrentPlayerMode 1))
  (Default|CallOnChangePlayerMode _output_get_2))

(fn GetCurrentPlayerMode
  (return (Variables|Default|GetCurrentPlayerMode)))